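; Behavior Tree node that picks the closest prey as the owning AI's target on each tick.
; It reads a PreyStructComponent from the Preys blackboard key and loops over its prey array, keeping the actor nearest to the owner.
; The result is written to the Target blackboard key.
; The stored Distance threshold is never reset in this graph, so it carries over between ticks.
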(event EventTick
  (params (OwnerActor :type Actor%20Object%20Reference) (DeltaSeconds :type Float%20%28single-precision%29))
  (Variables|Default|SetOwnerActor OwnerActor)
  ;[1 1 1] Get Prey Array
  (bind _asprey_struct_component (Utilities|Casting|CastToPreyStructComponent (Class|BTFunctionLibrary|GetBlackboardValueasObject (Variables|Preys|GetPreys))))
  (for _array_element (Variables|/Game/Swarm/Blueprints/Components/PreyStructComponent.PreyStructComponent_C|GetPrey%20Array%20Struct _asprey_struct_component)
    ;[1 1 1] Get Closest target
    (if (<= (Transformation|GetDistanceTo _array_element (Variables|Default|GetOwnerActor)) (Variables|Default|Getdistance))
      (Variables|Default|Setdistance (Transformation|GetDistanceTo _array_element (Variables|Default|GetOwnerActor)))
      (Variables|Default|SetnewTarget _array_element)))
  ;[1 1 1] Set Closest Target in BB
  (Class|BTFunctionLibrary|SetBlackboardValueasObject (Variables|Preys|GetTarget) (Variables|Default|GetnewTarget)))