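; Behavior Tree decorator for Swarm AI that checks whether the controlled pawn is aware of its target.
; It reads the Target actor and AwarenessRange from the Blackboard and passes when the distance between target and pawn is within that range.
; The test is purely distance-based, with no sight or perception check.
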(fn PerformConditionCheckAI
  (params (OwnerController :type AI%20Controller%20Object%20Reference) (ControlledPawn :type Pawn%20Object%20Reference))
  (bind _asactor (Utilities|Casting|CastToActor (Class|BTFunctionLibrary|GetBlackboardValueasObject (Variables|Default|GetTarget))))
  (if (<= (Transformation|GetDistanceTo _asactor ControlledPawn) (Class|BTFunctionLibrary|GetBlackboardValueasFloat (Variables|Default|GetAwareness%20Range)))
    (LocalVariables|Setis%20aware true)
    (else
      (LocalVariables|Setis%20aware false)))
  (return (LocalVariables|Getis%20aware)))