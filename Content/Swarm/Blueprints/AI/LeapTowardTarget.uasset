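; Behavior tree task that makes a swarm unit leap at its blackboard Target.
; It solves a fixed-speed ballistic toss velocity from the pawn to the target, failing the task when no arc exists.
; With a valid arc, a roughly even random roll either jumps and leaps with that velocity, starting the leap cooldown, or fakes it by starting only a fake-leap cooldown; both outcomes succeed.
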(event EventReceiveExecute
  (params (OwnerActor :type Actor%20Object%20Reference))
  (bind _asaicontroller (Utilities|Casting|CastToAIController OwnerActor))
  (bind _asactor (Utilities|Casting|CastToActor (Class|BTFunctionLibrary|GetBlackboardValueasObject (Variables|Default|GetTarget))))
  (bind (_tossvelocity _returnvalue) (Class|GameplayStatics|BlueprintSuggestProjectileVelocity (Transformation|GetActorLocation (Pawn|GetControlledPawn _asaicontroller)) (Transformation|GetActorLocation _asactor) 7.5e+02 0.0 "DoNotTrace" 0.0 false false))
  (if _returnvalue
    (CallFunction|SetSwarmPhysicon OwnerActor _tossvelocity)
    (AI|BehaviorTree|FinishExecute true)
    (else
      (AI|BehaviorTree|FinishExecute false))))

(fn SetSwarmPhysicon
  (params (Object :type Object%20Object%20Reference) (Toss%20Velocity :type Vector :default "0, 0, 0"))
  ;[1 1 1] Get Swarm Unit
  (bind _asaicontroller (Utilities|Casting|CastToAIController Object))
  (bind _asswarm_unit (Utilities|Casting|CastToSwarmUnit (Pawn|GetControlledPawn _asaicontroller)))
  ;[1 1 1] Random Chance Not To Leap
  (if (> (Math|Random|RandomIntegerinRange 0 100) 50)
    ;[1 1 1] Leap
    (Character|Jump _asswarm_unit)
    (Default|Leap _asswarm_unit Toss%20Velocity)
    (Default|StartLeapCooldown _asswarm_unit)
    (else
      ;[1 1 1] Fake Leap. Doesn't leap but start cooldown
      (Default|StartFakeLeapCooldown _asswarm_unit)))
  (return))