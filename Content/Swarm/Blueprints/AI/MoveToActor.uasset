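; Behavior tree task that sends the AI toward the current location of its Target blackboard actor.
; Execution caches the pawn's AI controller and opens a gate, so the move is issued on the following tick.
; It calls MoveToLocation on a position snapshot, then reports success and closes the gate without waiting for arrival.
; If Target is not an Actor, the task keeps retrying each tick without finishing.
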(event Custom|Close%20Gate
  (Utilities|FlowControl|Gate false) ; enters at Close
)

(event EventReceiveExecute
  (params (OwnerActor :type Actor%20Object%20Reference))
  (Utilities|Casting|CastToPawn OwnerActor)
  (bind _returnvalue (AI|GetAIController OwnerActor))
  (Utilities|FlowControl|Gate false) ; enters at Open
)

(event EventTick
  (params (OwnerActor :type Actor%20Object%20Reference) (DeltaSeconds :type Float%20%28single-precision%29))
  (Utilities|FlowControl|Gate false
    (:Exit
      (bind _asactor (Utilities|Casting|CastToActor (Class|BTFunctionLibrary|GetBlackboardValueasObject (Variables|Default|GetTarget))))
      (AI|Navigation|MovetoLocation (stale EventReceiveExecute _returnvalue) (Transformation|GetActorLocation _asactor) -1.0 false true false true)
      (AI|BehaviorTree|FinishExecute true)
      (CallFunction|CloseGate))))