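; A behavior tree task that initializes a swarm unit's blackboard for its AI.
; It stores the owner as SelfActor and the controlled SwarmUnit's prey component under PreyArray, exposing that list as an object key.
; It fills the component's array with every PreyController in the world, so the list holds controllers, without duplicates.
; It then writes fixed awareness and leap ranges, flags the blackboard as set and finishes successfully.
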(event EventReceiveExecute
  (params (OwnerActor :type Actor%20Object%20Reference))
  ;[1 1 1] Start
  (Utilities|FlowControl|Sequence
    (:then_0
      ;[1 1 1] Set SelfActor
      (Class|BTFunctionLibrary|SetBlackboardValueasObject (Variables|Default|GetSelf%20Actor) OwnerActor)
      ;[1 1 1] Get Minion Character
      (bind _asswarm_controller (Utilities|Casting|CastToSwarmController OwnerActor))
      (bind _asswarm_unit (Utilities|Casting|CastToSwarmUnit (Pawn|GetControlledPawn _asswarm_controller)))
      (bind _output_get (Variables|Default|SetSwarm%20Unit%20Reference _asswarm_unit))
      ;[1 1 1] Get Minion Character
      (Class|BTFunctionLibrary|SetBlackboardValueasObject (Variables|Default|GetPreyArray) (Variables|/Game/Swarm/Blueprints/Characters/SwarmUnit.SwarmUnit_C|GetPreyStructComponent _output_get)))
    (:then_1
      ;[1 1 1] Get Prey Characters
      (bind _outactors (Actor|GetAllActorsOfClass "/Game/Swarm/Blueprints/Characters/PreyController.PreyController_C"))
      (for _array_element _outactors
        (bind _asprey_struct_component (Utilities|Casting|CastToPreyStructComponent (Class|BTFunctionLibrary|GetBlackboardValueasObject (Variables|Default|GetPreyArray))))
        (Utilities|Array|AddUnique (Variables|/Game/Swarm/Blueprints/Components/PreyStructComponent.PreyStructComponent_C|GetPrey%20Array%20Struct _asprey_struct_component) _array_element)))
    (:then_2
      ;[1 1 1] Set Blabkboard is set to TRUE
      (Class|BTFunctionLibrary|SetBlackboardValueasFloat (Variables|Default|GetAwareness%20Range) 5e+03)
      (Class|BTFunctionLibrary|SetBlackboardValueasFloat (Variables|Default|GetLeap%20Range) 4.5e+02)
      (Class|BTFunctionLibrary|SetBlackboardValueasBool (Variables|Default|GetBB%20is%20Set) true)
      (AI|BehaviorTree|FinishExecute true))))