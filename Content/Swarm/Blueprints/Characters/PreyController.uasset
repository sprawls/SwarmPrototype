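; PreyController is the controller for the prey player in a swarm game, handling sprint input and debug keys.
; The Sprint action toggles IsSprinting on MainPlayerState, fetched through a cast helper that logs an error on failure.
; Debug keys call RemoveLeapDebug on every SwarmUnit actor and reload the ThirdPersonExampleMap level.
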(event Input|KeyboardEvents|R
  ;[1 1 1] DEBUG : RESET MAP
  (:Pressed
    (Game|OpenLevel(byName) "ThirdPersonExampleMap")))

(event Input|KeyboardEvents|T
  ;[1 1 1] DEBUG : REMOVE LEAP
  (:Pressed
    (bind _outactors (Actor|GetAllActorsOfClass "/Game/Swarm/Blueprints/Characters/SwarmUnit.SwarmUnit_C"))
    (for _array_element _outactors
      (Default|RemoveLeapDebug _array_element))))

(event Input|ActionEvents|InputActionSprint
  (bind _playerstate (Accessors|GetPlayerState))
  (:Pressed
    (Variables|/Game/Swarm/Blueprints/Players/MainPlayerState.MainPlayerState_C|SetisSprinting _playerstate true))
  (:Released
    (Variables|/Game/Swarm/Blueprints/Players/MainPlayerState.MainPlayerState_C|SetisSprinting _playerstate false)))

(event Input|ActionEvents|InputActionUse)

(fn ConstructionScript
  (|CallParentFunction))

(fn GetPlayerState
  (bind _asmain_player_state (Utilities|Casting|CastToMainPlayerState (Variables|Default|GetPlayerState))
    (:then
      (return _asmain_player_state))
    (:CastFailed
      (Class|VisualLoggerKismetLibrary|LogText "PreyController::GetPlayerState - Cast failed!" "Blueprint Errors"))))