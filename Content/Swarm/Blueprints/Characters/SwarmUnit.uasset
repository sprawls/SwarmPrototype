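; SwarmUnit is a single swarm creature ("grubbler") that can leap and latch onto prey.
; Leap launches the capsule with physics velocity and ignores a trace channel to avoid high-velocity collisions between grubblers.
; Cooldown timers gate leaping and call StopLeaping to restore rotation, physics and collision.
; Overlapping a PreyController replaces the unit with a scaled, randomly rotated AttachedSwarmUnit on a random mesh socket.
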(event Custom|Remove%20Leap%20Debug
  ;[1 1 1] DEBUG : Remove Leap
  (Utilities|Time|SetTimerbyEvent (delegate Custom|Debug%20Disable%20Leap) 0.5 true))

(event Custom|StartFakeLeapCooldown
  ;[1 1 1] Leap Cooldown
  (Variables|Default|SetCanLeap false)
  (Utilities|Time|SetTimerbyFunctionName 0 "EndLeapCooldown" (/ (Variables|Default|GetLeap%20Cooldown%20Time) 1.0)))

(event Custom|StartLeapCooldown
  ;[1 1 1] Leap Cooldown
  (Variables|Default|SetCanLeap false)
  (Variables|Default|SetisLeaping true)
  (Utilities|Time|SetTimerbyFunctionName 0 "EndLeapCooldown" (Variables|Default|GetLeap%20Cooldown%20Time)))

(event Custom|EndLeapCooldown
  ;[1 1 1] Leap Cooldown
  (Variables|Default|SetCanLeap true)
  (CallFunction|StopLeaping))

(event Custom|Debug%20Disable%20Leap
  ;[1 1 1] DEBUG : Remove Leap
  (Variables|Default|SetCanLeap false))

(event EventBeginPlay)

(event EventActorBeginOverlap
  (params (OtherActor :type Actor%20Object%20Reference))
  ;[1 1 1] Disable swarm unit and Attach to socket
  (bind _asprey_controller (Utilities|Casting|CastToPreyController OtherActor))
  (bind _returnvalue (Game|SpawnActorfromClass "/Game/Swarm/Blueprints/Characters/AttachedSwarmUnit.AttachedSwarmUnit_C" (Transformation|GetActorTransform) true 0))
  (Class|Actor|AttachRootComponentto _returnvalue (Variables|/Script/Engine.Character|GetMesh _asprey_controller) (Utilities|String|StringToName (Utilities|String|Append "SwarmSocket_" (Utilities|String|ToString(Integer) (Math|Random|RandomIntegerinRange 0 7)))) "SnapToTarget" true)
  ;[1 1 1] Fix unit size
  (Transformation|SetActorScale3D _returnvalue "0.250000,0.250000,0.250000")
  ;[1 1 1] Set Random Rotation
  (Transformation|SetActorRotation _returnvalue (Math|Random|RandomRotator true))
  ;[1 1 1] Destroy This Actor
  (Actor|DestroyActor))

(fn ConstructionScript)

(fn StopLeaping
  (Variables|Default|SetisLeaping false)
  (Physics|SetSimulatePhysics false)
  (Transformation|SetActorRotation "0, 0, 0")
  (Collision|SetCollisionResponsetoChannel (Variables|Collision|GetCapsuleComponent) "ECC_GameTraceChannel1" "ECR_Block")
  (return))

(fn Leap
  (params (Velocity :type Vector :default "0, 0, 0"))
  (bind _capsulecomponent (Variables|Collision|GetCapsuleComponent))
  (Physics|SetSimulatePhysics _capsulecomponent true)
  (Physics|SetPhysicsLinearVelocity _capsulecomponent Velocity false "None")
  (Collision|SetCollisionResponsetoChannel "ECC_GameTraceChannel1" "ECR_Ignore") ; Remove collision with other grubbler since this causes them to collide together and gain very high velocity
)